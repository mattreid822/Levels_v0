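; BP_FSARevolver is a futuristic revolver that fires projectiles and reloads.
; BeginPlay snaps six bullet components to sockets on the gun mesh.
; Fire counts shots, starts the firing montage only on the first, then after a short delay spawns BP_FSARevProjectile at the supplied transform with muzzle sound and barrel flame.
; Reloading plays its montage and resets the counter, so the next shot restarts the firing montage.
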(event Custom|Fire
  (params (SpawnTransform :type Transform))
  (bind _arrow1 (Variables|Default|GetArrow1))
  ;[1 1 1] Firing
  (bind _result (Math|Integer|IncrementInt (Variables|Default|GetShoots))
    (:%20%20
      (if (== _result 1) ; Play the montage only ones/per six shoot, triggered by the first shoot, after pause the montage until new fire input comes
        (Animation|Montage|MontagePlay (Components|SkeletalMesh|GetAnimInstance (Variables|Default|GetFSARevolver)) "/Game/FuturisticRevolver/Animations/FSARevolver/FSARev_GunFire_Montage.FSARev_GunFire_Montage" 1.0 "MontageLength" 0.0) ; Revolver firing montage
      )
      (Utilities|FlowControl|Delay 0.1) ; Little delay after firing, looks more realistic
      (Game|SpawnActorfromClass "/Game/FuturisticRevolver/Blueprints/BP_FSARevProjectile.BP_FSARevProjectile_C" SpawnTransform "AdjustIfPossibleButAlwaysSpawn" 0 0) ; Spawn the bullet
      (Audio|PlaySoundatLocation "/Game/FuturisticRevolver/Sounds/Cue/SC_FSARevShoot01.SC_FSARevShoot01" (Transformation|GetSocketLocation (Variables|Default|GetFSARevolver) "FSA_Revolver_muzzleSocket"))
      (Effects|SpawnEmitteratLocation "/Game/FuturisticRevolver/Particles/PS_FSARevBarrelFlame.PS_FSARevBarrelFlame" (Transformation|GetWorldLocation _arrow1) (Transformation|GetWorldRotation _arrow1)) ; Spawn the firing effect for the barrel
    )))

(event Custom|Reloading
  ;[1 1 1] Reloading
  (Animation|Montage|MontagePlay (Components|SkeletalMesh|GetAnimInstance (Variables|Default|GetFSARevolver)) "/Game/FuturisticRevolver/Animations/FSARevolver/FSARev_GunReloading_Montage.FSARev_GunReloading_Montage" 1.0 "MontageLength" 0.0) ; Reloading one bullet montage
  (Variables|Default|SetShoots 0))

(event EventBeginPlay
  (bind _fsarevolver (Variables|Default|GetFSARevolver))
  ;[1 1 1] Attach bullets to gun
  (Transformation|AttachComponentToComponent (Variables|Default|GetBullet1) _fsarevolver "FSA_bullet_1Socket" "SnapToTarget" "SnapToTarget" "SnapToTarget" true)
  (Transformation|AttachComponentToComponent (Variables|Default|GetBullet2) _fsarevolver "FSA_bullet_2Socket" "SnapToTarget" "SnapToTarget" "SnapToTarget" true)
  (Transformation|AttachComponentToComponent (Variables|Default|GetBullet3) _fsarevolver "FSA_bullet_3Socket" "SnapToTarget" "SnapToTarget" "SnapToTarget" true)
  (Transformation|AttachComponentToComponent (Variables|Default|GetBullet4) _fsarevolver "FSA_bullet_4Socket" "SnapToTarget" "SnapToTarget" "SnapToTarget" true)
  (Transformation|AttachComponentToComponent (Variables|Default|GetBullet5) _fsarevolver "FSA_bullet_5Socket" "SnapToTarget" "SnapToTarget" "SnapToTarget" true)
  (Transformation|AttachComponentToComponent (Variables|Default|GetBullet6) _fsarevolver "FSA_bullet_6Socket" "SnapToTarget" "SnapToTarget" "SnapToTarget" true))

(fn ConstructionScript)